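; BP_MyPaperCharacter is a Paper2D player character for a side-scrolling game, driven by Enhanced Input.
; BeginPlay adds the 2D mapping context and binds the jump-apex event, which only prints a debug message.
; Walking moves along world X, swaps walk and idle flipbooks, and mirrors the sprite by flipping its X scale.
; Jumping briefly shows an explosion flipbook before idle, while OnJumped enables apex notification.
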(event Custom|OnReachedJumpApex_Event
  (Development|PrintString "apex"))

(event Input|EnhancedActionEvents|EnhancedInputActionIA_Walk2D
  (params (ActionValue :type Float%20%28double-precision%29) (ElapsedSeconds :type Float%20%28double-precision%29) (TriggeredSeconds :type Float%20%28double-precision%29) (InputAction :type Input%20Action%20Object%20Reference :default "/Game/2dGame/IA_Walk2D.IA_Walk2D"))
  (:Triggered
    (Pawn|Input|AddMovementInput (Math|Vector|MakeVector ActionValue 0.0 0.0) 0.5 false)
    (Sprite|SetFlipbook (Variables|Default|GetSprite) "/Game/2dGame/Character/PF_Walking.PF_Walking")
    (Transformation|SetWorldScale3D (Variables|Default|GetSprite) (Math|Vector|MakeVector (* (Math|Float|Sign(Float) ActionValue) -1.0) 1.0 1.0)))
  (:Completed
    (Sprite|SetFlipbook (Variables|Default|GetSprite) "/Game/2dGame/Character/PF_Idle.PF_Idle")))

(event Input|EnhancedActionEvents|EnhancedInputActionIA_Jump2D
  (params (ActionValue :type Boolean) (ElapsedSeconds :type Float%20%28double-precision%29) (TriggeredSeconds :type Float%20%28double-precision%29) (InputAction :type Input%20Action%20Object%20Reference :default "/Game/2dGame/IA_Jump2D.IA_Jump2D"))
  (Character|Jump)
  (Sprite|SetFlipbook (Variables|Default|GetSprite) "/Game/2dGame/Explosion/PF_Explosion.PF_Explosion")
  (Utilities|FlowControl|Delay 0.4)
  (Sprite|SetFlipbook (Variables|Default|GetSprite) "/Game/2dGame/Character/PF_Idle.PF_Idle"))

(event EventOnJumped
  (Variables|/Script/Engine.CharacterMovementComponent|SetbNotifyApex (Variables|Character|GetCharacterMovement) true))

(event Collision|EventActorBeginOverlap
  (params (OtherActor :type Actor%20Object%20Reference)))

(event EventBeginPlay
  (Input|AddMappingContext (PlayerController|LocalPlayerSubsystems|GetEnhancedInputLocalPlayerSubsystem self) "/Game/2dGame/IMC_2D.IMC_2D" 0 "(bIgnoreAllPressedKeysUntilRelease=True,bForceImmediately=False,bNotifyUserSettings=False)")
  (EventDispatchers|AssignOnReachedJumpApex (delegate Custom|OnReachedJumpApex_Event)))

(fn ConstructionScript)